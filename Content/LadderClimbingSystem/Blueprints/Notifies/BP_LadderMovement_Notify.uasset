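; Animation notify for the ladder climbing system that advances the owner's climb step by step from the animation.
; On the locally controlled instigator it finds the standard or FPTP ladder component and reads its ladder data via interface.
; While axis input is non-zero, it alternates left and right climb states and sends move up or down messages.
; Slide keeps sending slide down; idle states do nothing.
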(fn ReceivedNotify
  (params (MeshComp :type Skeletal%20Mesh%20Component%20Object%20Reference) (Animation :type Anim%20Sequence%20Base%20Object%20Reference) (EventReference :type Anim%20Notify%20Event%20Reference%20Structure%20%28by%20ref%29))
  ;[0 0 0] Check if instigator is valid, Set a local ref to the instigator
  (bind _instigator (Variables|/Script/Engine.Actor|GetInstigator (Components|GetOwner MeshComp))
    (:then
      (LocalVariables|SetLocalInstigatorRef _instigator)
      ;[0 0 0] Check if Locally controlled
      (if (Pawn|IsLocallyControlled (LocalVariables|GetLocalInstigatorRef))
        ;[0 0 0 1 15] Set reference to ladder component attached to player
        (Utilities|IsValid (Actor|GetComponentbyClass (LocalVariables|GetLocalInstigatorRef) "/Game/LadderClimbingSystem/Blueprints/Components/BPC_LadderClimbingComponent.BPC_LadderClimbingComponent_C")
          (:Is%20Valid
            (LocalVariables|SetLocalLadderComponentRef (Actor|GetComponentbyClass (LocalVariables|GetLocalInstigatorRef) "/Game/LadderClimbingSystem/Blueprints/Components/BPC_LadderClimbingComponent.BPC_LadderClimbingComponent_C")))
          (:Is%20Not%20Valid
            (LocalVariables|SetLocalLadderComponentRef (Actor|GetComponentbyClass (LocalVariables|GetLocalInstigatorRef) "/Game/LadderClimbingSystem/Blueprints/Components/BPC_FPTP_LadderClimbingComponent.BPC_FPTP_LadderClimbingComponent_C"))))
        ;[0 0 0] Set a value for the Ladder Data to be used in the notify
        (bind _ladderdata (Class|BPILadderClimbingInterface|BPIGetLadderData(Message) (LocalVariables|GetLocalLadderComponentRef)))
        (LocalVariables|SetLocalLadderData _ladderdata)
        ;[0 0 0] Check if Axis value does not equal 0
        (if (!= (Utilities|Struct|BreakST_LadderData (LocalVariables|GetLocalLadderData)) 0.0)
          ;[0 0 0 1 15] Check current Movement State
          (switch Utilities|FlowControl|Switch|SwitchonE_LadderMovementState (Utilities|Struct|BreakST_LadderData (LocalVariables|GetLocalLadderData))
            (:NewEnumerator12
              ;[0 0 0 1 15] Set Next Ladder Movement State and Send a Message to the Move Up Event in the Ladder Component.
              (Class|BPILadderClimbingInterface|BPISetLadderMovementState(Message) (LocalVariables|GetLocalLadderComponentRef) "NewEnumerator13")
              (Class|BPILadderClimbingInterface|BPILadderMoveUp(Message) (LocalVariables|GetLocalLadderComponentRef) :!label _label))
            (:NewEnumerator13
              (Class|BPILadderClimbingInterface|BPISetLadderMovementState(Message) (LocalVariables|GetLocalLadderComponentRef) "NewEnumerator12")
              (goto _label))
            (:NewEnumerator14
              ;[0 0 0 1 15] Set Next Ladder Movement State and Send a Message to the Move Down Event in the Ladder Component.
              (Class|BPILadderClimbingInterface|BPISetLadderMovementState(Message) (LocalVariables|GetLocalLadderComponentRef) "NewEnumerator15")
              (Class|BPILadderClimbingInterface|BPILadderMoveDown(Message) (LocalVariables|GetLocalLadderComponentRef)))
            (:NewEnumerator15
              (Class|BPILadderClimbingInterface|BPISetLadderMovementState(Message) (LocalVariables|GetLocalLadderComponentRef) "NewEnumerator14")
              (Class|BPILadderClimbingInterface|BPILadderMoveDown(Message) (LocalVariables|GetLocalLadderComponentRef)))
            (:NewEnumerator16
              (return false))
            (:NewEnumerator17
              (return false))
            (:NewEnumerator18
              (Class|BPILadderClimbingInterface|BPISetLadderMovementState(Message) (LocalVariables|GetLocalLadderComponentRef) "NewEnumerator18")
              (Class|BPILadderClimbingInterface|BPISlideDown(Message) (LocalVariables|GetLocalLadderComponentRef))))
          (return true))))
    (:else)))