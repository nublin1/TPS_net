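; BP_Director is a director actor that tracks the level's zombies and handles spawn requests from horde spawners.
; On BeginPlay it registers existing zombies, binds their health components' killed delegates, and subscribes to each spawner's spawn request.
; OnZombieSpawnRequested spawns zombies at random reachable points near a given location and adds them to the list, without binding their killed delegate.
; Tick prints the zombie count for debugging.
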(event Custom|Kill
  (params (KilledActor :type Actor%20Object%20Reference))
  (Class|Director|OnZombieKilled (.AsBP%20NPCCharacter (Utilities|Casting|CastToBP_NPCZombie KilledActor))))

(event EventBeginPlay
  (Utilities|FlowControl|Sequence
    (:then_0
      (bind _outactors (Actor|GetAllActorsOfClass "/Game/ThirdPerson/Blueprints/NPC/BP_NPCZombie.BP_NPCZombie_C"))
      (for _array_element _outactors
        (Utilities|Array|Add (Variables|Default|GetZombies) _array_element)
        (bind _asihealth_interface (Utilities|Casting|CastToIHealthInterface _array_element))
        (Utilities|IsValid (Class|IHealthInterface|GetHealthComponent _asihealth_interface)
          (:Is%20Valid
            (EventDispatchers|BindEventtoOnKilledDelegate (Class|IHealthInterface|GetHealthComponent _asihealth_interface) (delegate Custom|Kill))))))
    (:then_1
      (bind _outactors_2 (Actor|GetAllActorsOfClass "/Game/Director/BP_HorderSpawner.BP_HorderSpawner_C"))
      (for _array_element_2 _outactors_2
        (CallFunction|OnHorderSpawnerSpawned _array_element_2)))))

(event Collision|EventActorBeginOverlap
  (params (OtherActor :type Actor%20Object%20Reference)))

(event EventTick
  (params (DeltaSeconds :type Float%20%28single-precision%29))
  (Development|PrintString (Utilities|String|Append "Num Zombied: " (Utilities|String|ToString(Integer) (Utilities|Array|Length (Variables|Default|GetZombies)))) true false "(R=0.000000,G=0.660000,B=1.000000,A=1.000000)" 0.0))

(fn ConstructionScript)

(fn OnZombieSpawned
  (params (Zombie :type NPC%20Character%20Object%20Reference))
  (Utilities|Array|Add (Variables|Default|GetZombies) (.AsBP%20NPCCharacter (Utilities|Casting|CastToBP_NPCZombie Zombie))))

(fn OnHorderSpawnerSpawned
  (params (HorderSpawner :type BP%20Horder%20Spawner%20Object%20Reference))
  (Utilities|Array|Add (Variables|Default|GetHorderSpawners) HorderSpawner)
  (EventDispatchers|BindEventtoRequestSpawn HorderSpawner (EventDispatchers|CreateEvent :!event OnZombieSpawnRequested)))

(fn OnZombieSpawnRequested
  (params (Count :type Integer) (Location :type Vector))
  (for _index (range 1 Count)
    (bind _returnvalue (Game|SpawnActorfromClass "/Game/ThirdPerson/Blueprints/NPC/BP_NPCZombie.BP_NPCZombie_C" (Math|Transform|MakeTransform (+ (.RandomLocation (AI|Navigation|GetRandomReachablePointinRadius Location 2e+02 0 0)) "0.000000,0.000000,90.000000") "0, 0, 0" "1.000000,1.000000,1.000000") "Undefined" "MultiplyWithRoot" 0 0))
    (CallFunction|OnZombieSpawned _returnvalue)))