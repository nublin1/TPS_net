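; BP_HitNotifyState is an animation notify state that marks the hit-detection window in a zombie combat animation.
; On begin it clears the combat component's already-hit targets, then calls HitDetect on that component every tick of the window.
; It reaches the component through ZombieCombatInterface on the mesh's owner, so owners without the interface are ignored.
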(fn ReceivedNotifyTick
  (params (MeshComp :type Skeletal%20Mesh%20Component%20Object%20Reference) (Animation :type Anim%20Sequence%20Base%20Object%20Reference) (FrameDeltaTime :type Float%20%28single-precision%29) (EventReference :type Anim%20Notify%20Event%20Reference%20Structure%20%28by%20ref%29))
  (bind _returnvalue (Components|GetOwner MeshComp))
  (if (Utilities|DoesObjectImplementInterface _returnvalue "/Script/TPS_net.ZombieCombatInterface")
    (bind _returnvalue_2 (Class|ZombieCombatInterface|GetZombieCombatComponent(Message) _returnvalue))
    (Class|ZombieCombatComponent|HitDetect _returnvalue_2))
  (return false))

(fn ReceivedNotifyBegin
  (params (MeshComp :type Skeletal%20Mesh%20Component%20Object%20Reference) (Animation :type Anim%20Sequence%20Base%20Object%20Reference) (TotalDuration :type Float%20%28single-precision%29) (EventReference :type Anim%20Notify%20Event%20Reference%20Structure%20%28by%20ref%29))
  (bind _returnvalue (Components|GetOwner MeshComp))
  (if (Utilities|DoesObjectImplementInterface _returnvalue "/Script/TPS_net.ZombieCombatInterface")
    (bind _returnvalue_2 (Class|ZombieCombatInterface|GetZombieCombatComponent(Message) _returnvalue))
    (Class|ZombieCombatComponent|ClearAlreadyHitTargets _returnvalue_2)
    (return false)))