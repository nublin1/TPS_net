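; BP_ProceduralLadder is a climbable ladder that builds itself to a set height and manages where characters enter and exit it.
; The construction script stretches the poles, adds instanced rungs and optional screws, and positions the top markers and exit box.
; Trigger boxes check the character's state tag and sliding flag, then send messages to register top or bottom entry or exit at motion-warp points.
; The top return box acts only on authority.
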(event OnComponentBeginOverlap(EnterBox)
  (params (OverlappedComponent :type Primitive%20Component%20Object%20Reference) (OtherActor :type Actor%20Object%20Reference) (OtherComp :type Primitive%20Component%20Object%20Reference) (OtherBodyIndex :type Integer) (bFromSweep :type Boolean) (SweepResult :type Hit%20Result%20Structure%20%28by%20ref%29))
  (bind (_asbp_third_person_character _bsuccess) (Utilities|Casting|CastToBP_ThirdPersonCharacter OtherActor))
  (bind _motionwarplocation_down (Variables|Default|GetMotionWarpLocation_Down))
  (bind _returnvalue (Transformation|GetWorldLocation _motionwarplocation_down))
  (bind _statemachine_movemant (Variables|/Script/TPS_net.PlayerCharacter|GetStateMachine_Movemant _asbp_third_person_character))
  (bind _currentstatetag (Variables|/Script/TPS_net.StateMachineComponent|GetCurrentStateTag _statemachine_movemant))
  ;[1 1 1] Can interact with ladder
  (Development|PrintString (Utilities|String|EnumtoString (Networking|GetLocalRole)) true true "(R=0.000000,G=0.660000,B=1.000000,A=1.000000)" 1.0)
  (if _bsuccess
    (if (!= _currentstatetag "(TagName=\"PlayerStates.Ladder.OnLadder\")")
      (Class|BPILadder|SetLadderInteraction(Message) OtherActor self)
      (Collision|SetCollisionEnabled (Variables|Default|GetExitBox) "QueryAndPhysics")
      (bind _asbp_third_person_character_2 (Utilities|Casting|CastToBP_ThirdPersonCharacter OtherActor))
      (Variables|/Game/ThirdPerson/Blueprints/BP_ThirdPersonCharacter.BP_ThirdPersonCharacter_C|SetIsUpLadderEntry _asbp_third_person_character_2 false)
      (elif (and (== _currentstatetag "(TagName=\"PlayerStates.Ladder.OnLadder\")") (not (Variables|/Game/ThirdPerson/Blueprints/BP_ThirdPersonCharacter.BP_ThirdPersonCharacter_C|GetLadderSliding _asbp_third_person_character)))
        (Class|BPILadder|ExitLadder(Message) OtherActor _returnvalue _returnvalue false)))))

(event OnComponentBeginOverlap(ExitBox)
  (params (OverlappedComponent :type Primitive%20Component%20Object%20Reference) (OtherActor :type Actor%20Object%20Reference) (OtherComp :type Primitive%20Component%20Object%20Reference) (OtherBodyIndex :type Integer) (bFromSweep :type Boolean) (SweepResult :type Hit%20Result%20Structure%20%28by%20ref%29))
  (bind (_asbp_third_person_character _bsuccess) (Utilities|Casting|CastToBP_ThirdPersonCharacter OtherActor))
  ;[1 1 1] Comment
  (if _bsuccess
    (if (== (Variables|/Script/TPS_net.StateMachineComponent|GetCurrentStateTag (Variables|/Script/TPS_net.PlayerCharacter|GetStateMachine_Movemant _asbp_third_person_character)) "(TagName=\"PlayerStates.Ladder.OnLadder\")")
      (Class|BPILadder|ExitLadder(Message) OtherActor (+ (Transformation|GetWorldLocation (Variables|Default|GetDefaultSceneRoot)) (Math|Vector|MakeVector 0.0 0.0 (* (Variables|Default|GetLedderHeight) 1e+02))) (- (Transformation|GetWorldLocation (Variables|Default|GetMotionWarpLocation_Up)) "") true)
      (Collision|SetCollisionEnabled (Variables|Default|GetReturnBox) "QueryAndPhysics")
      (Class|BPILadder|SetLadderInteraction(Message) OtherActor (Variables|Default|GetEmptyActor)))))

(event OnComponentBeginOverlap(ReturnBox)
  (params (OverlappedComponent :type Primitive%20Component%20Object%20Reference) (OtherActor :type Actor%20Object%20Reference) (OtherComp :type Primitive%20Component%20Object%20Reference) (OtherBodyIndex :type Integer) (bFromSweep :type Boolean) (SweepResult :type Hit%20Result%20Structure%20%28by%20ref%29))
  ;[1 1 1] Comment
  (Networking|SwitchHasAuthority
    (:Authority
      (bind _asbp_third_person_character (Utilities|Casting|CastToBP_ThirdPersonCharacter OtherActor))
      (Utilities|FlowControl|Sequence
        (:then_0
          (Class|BPILadder|SetLadderInteraction(Message) OtherActor self))
        (:then_1
          (Collision|SetCollisionEnabled (Variables|Default|GetExitBox) "QueryAndPhysics"))
        (:then_2
          (Utilities|IsValid _asbp_third_person_character
            (:Is%20Valid
              (if (!= (Variables|/Script/TPS_net.StateMachineComponent|GetCurrentStateTag (Variables|/Script/TPS_net.PlayerCharacter|GetStateMachine_Movemant _asbp_third_person_character)) "(TagName=\"PlayerStates.Ladder.OnLadder\")")
                (Variables|/Game/ThirdPerson/Blueprints/BP_ThirdPersonCharacter.BP_ThirdPersonCharacter_C|SetIsUpLadderEntry _asbp_third_person_character true)))))))))

(event OnComponentEndOverlap(EnterBox)
  (params (OverlappedComponent :type Primitive%20Component%20Object%20Reference) (OtherActor :type Actor%20Object%20Reference) (OtherComp :type Primitive%20Component%20Object%20Reference) (OtherBodyIndex :type Integer))
  (bind _returnvalue (Game|GetPlayerCharacter 0))
  (if (== OtherActor _returnvalue)
    (CallFunction|ExitEnteringLadderZone (.AsBP%20Third%20Person%20Character (Utilities|Casting|CastToBP_ThirdPersonCharacter _returnvalue)))))

(event OnComponentEndOverlap(ExitBox)
  (params (OverlappedComponent :type Primitive%20Component%20Object%20Reference) (OtherActor :type Actor%20Object%20Reference) (OtherComp :type Primitive%20Component%20Object%20Reference) (OtherBodyIndex :type Integer))
  (bind _returnvalue (Game|GetPlayerCharacter 0))
  (if (== OtherActor _returnvalue)
    (CallFunction|ExitEnteringLadderZone (.AsBP%20Third%20Person%20Character (Utilities|Casting|CastToBP_ThirdPersonCharacter _returnvalue)))))

(event OnComponentBeginOverlap(SlideExitBox)
  (params (OverlappedComponent :type Primitive%20Component%20Object%20Reference) (OtherActor :type Actor%20Object%20Reference) (OtherComp :type Primitive%20Component%20Object%20Reference) (OtherBodyIndex :type Integer) (bFromSweep :type Boolean) (SweepResult :type Hit%20Result%20Structure%20%28by%20ref%29))
  (bind (_asbp_third_person_character _bsuccess) (Utilities|Casting|CastToBP_ThirdPersonCharacter OtherActor))
  (bind _motionwarplocation_down (Variables|Default|GetMotionWarpLocation_Down))
  (bind _returnvalue (Transformation|GetWorldLocation _motionwarplocation_down))
  (if _bsuccess
    (if (and (== (Variables|/Script/TPS_net.StateMachineComponent|GetCurrentStateTag (Variables|/Script/TPS_net.PlayerCharacter|GetStateMachine_Movemant _asbp_third_person_character)) "(TagName=\"PlayerStates.Ladder.OnLadder\")") (Variables|/Game/ThirdPerson/Blueprints/BP_ThirdPersonCharacter.BP_ThirdPersonCharacter_C|GetLadderSliding _asbp_third_person_character))
      (Class|BPILadder|ExitLadder(Message) OtherActor _returnvalue _returnvalue false))))

(event Custom|ExitEnteringLadderZone
  (params (Actor :type BP%20Third%20Person%20Character%20Object%20Reference))
  (if (== (Variables|/Script/TPS_net.StateMachineComponent|GetCurrentStateTag (Variables|/Script/TPS_net.PlayerCharacter|GetStateMachine_Movemant Actor)) "(TagName=\"PlayerStates.Ladder.OnLadder\")")
    _))

(event EventBeginPlay)

(event Collision|EventActorBeginOverlap
  (params (OtherActor :type Actor%20Object%20Reference)))

(event EventTick
  (params (DeltaSeconds :type Float%20%28single-precision%29)))

(fn ConstructionScript
  (bind _ledderheight (Variables|Default|GetLedderHeight))
  (bind _ledderheight_2 (Variables|Default|GetLedderHeight))
  (bind _returnvalue (Math|Vector|MakeVector 0.1 0.1 _ledderheight))
  (bind _returnvalue_2 (* _ledderheight_2 1e+02))
  (bind _returnvalue_3 (* _ledderheight 1e+02))
  (bind _returnvalue_4 (/ _returnvalue_3 2.0))
  (bind _returnvalue_5 (Math|Vector|MakeVector 0.0 0.0 _returnvalue_4))
  (Class|SceneComponent|AddLocalTransform (Variables|Default|GetLeftLadderPole) (Math|Transform|MakeTransform _returnvalue_5 "0, 0, 0" _returnvalue) false false)
  (Class|SceneComponent|AddLocalTransform (Variables|Default|GetRightLadderPole) (Math|Transform|MakeTransform _returnvalue_5 "0, 0, 0" _returnvalue) false false)
  (Transformation|SetRelativeLocation (Variables|Default|GetExitBox) (Math|Vector|MakeVector 0.0 0.0 (+ _returnvalue_2 (Variables|Default|GetExitBoxOffset))) false false)
  (Transformation|SetRelativeLocation (Variables|Default|GetLadderExitArea) (Math|Vector|MakeVector 0.0 0.0 (+ _returnvalue_2 (Variables|Default|GetLadderExitAreaOffset))) false false)
  (Transformation|SetRelativeLocation (Variables|Default|GetLadderBeginningUpPosition) (Math|Vector|MakeVector -3e+01 0.0 (- (* (Variables|Default|GetLedderHeight) 1e+02) (LocalVariables|GetBeginningUpPositionOffset))) false false)
  (Utilities|FlowControl|Sequence
    (:then_0
      (while (< (Variables|Default|GetCompareHeight) (* (Variables|Default|GetLedderHeight) 1e+02))
        (Utilities|AddBarsandScrews)))
    (:then_1
      (Utilities|SetExitPoints))))