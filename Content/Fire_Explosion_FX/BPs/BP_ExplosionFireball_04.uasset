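; BP_ExplosionFireball_04 is an explosion fireball effect actor that pairs a particle system with a point light.
; The construction script applies a shared PColor to both the particle color parameter and the light color.
; On BeginPlay, a timeline plays from the start and drives the light's intensity over the effect's lifetime.
; Particle setters for brightness, scattering and max output exist but are never executed.
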(event EventBeginPlay
  (bind _intensity (Timeline|Timeline_0 PlayFromStart)
    (:Update
      (Rendering|Components|Light|SetIntensity (Variables|Default|GetPointLight) _intensity))))

(fn ConstructionScript
  (bind _pcolor (Variables|Default|GetPColor))
  (Effects|Components|ParticleSystem|SetColorParameter (Variables|Default|GetParticleSystem) "PColor" _pcolor)
  (Rendering|Components|Light|SetLightColor (Variables|Default|GetPointLight) _pcolor true))