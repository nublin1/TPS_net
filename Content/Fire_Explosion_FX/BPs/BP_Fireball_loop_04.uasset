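; BP_Fireball_loop_04 is an effect actor that repeatedly plays the PS_fireball_04 particle explosion with a matching light animation.
; From BeginPlay, Timeline_0 acts as a loop timer, restarting itself on each finish and spawning the emitter at the actor's transform.
; Each cycle also restarts Timeline_1, whose curve drives the point light's intensity.
; The construction script tints that light from the PColor variable.
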(event EventBeginPlay
  (bind _returnvalue (Transformation|GetActorTransform))
  (Timeline|Timeline_0 PlayFromStart
    (:Finished
      (Utilities|FlowControl|Sequence
        (:then_0
          (Effects|SpawnEmitteratLocation "/Game/Fire_Explosion_FX/ParticleSystems/PS_fireball_04.PS_fireball_04" (.location _returnvalue) (.rotation _returnvalue) (.scale _returnvalue))
          (Timeline|Timeline_0 PlayFromStart))
        (:then_1
          (bind _intensity (Timeline|Timeline_1 PlayFromStart)
            (:Update
              (Rendering|Components|Light|SetIntensity (Variables|Default|GetPointLight) _intensity))))))))

(fn ConstructionScript
  (Rendering|Components|Light|SetLightColor (Variables|Default|GetPointLight) (Variables|Default|GetPColor) true))